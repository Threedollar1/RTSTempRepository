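; BP_Farm is a farm building for the RTS builder template that generates resources and can be upgraded.
; It overrides HUD button events to start generation, upgrade the building with a wood cost and faster, larger output, or clear the generating flag.
; Generation and upgrade logic come from calls defined outside these graphs; the farm supplies upgrade tuning and tells the RTS pawn which HUD panels to show.
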(event EventButton3Clicked
  (Variables|Default|SetIs%20Generating false))

(event EventBeginPlay
  (|CallParentFunction))

(event EventActorBeginOverlap
  (params (OtherActor :type Actor%20Object%20Reference)))

(event EventTick
  (params (DeltaSeconds :type Float%20%28single-precision%29))
  (|CallParentFunction 0.0))

(event EventSetHUDVisibilitys
  (Default|SetHUDVisibilitys (Variables|Default|GetRTS%20Pawn) "Hidden" "Visible" "Hidden" "Hidden" "Hidden" "Hidden" "Visible" "Hidden" "Hidden" "Visible"))

(event EventButton1Clicked
  (CallFunction|GenerateResources))

(event EventButton2Clicked
  (CallFunction|UpgradeBuilding 3 0 0.0 0 0.9 2 0.0 0.0 0.0 0 250))

(fn ConstructionScript
  (|CallParentFunction))